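; Gameplay ability for a ranged attack that fires a projectile at the avatar's combat target.
; It turns the avatar toward the target, then plays a random tagged attack montage, both via messages to the avatar.
; A gameplay event matching the montage's tag triggers the projectile spawn and a debug sphere at the combat socket.
; The ability ends when the montage completes, is interrupted or is cancelled.
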(event `self.K2_ActivateAbility`
  (bind _returnvalue (`self.GetAvatarActorFromActorInfo`))
  (bind _returnvalue_2 (message `EnemyInterface.GetCombatTarget` _returnvalue))
  (bind _returnvalue_3 (`Actor.K2_GetActorLocation` _returnvalue_2))
  (message `CombatInterface.UpdateFacingTarget` _returnvalue _returnvalue_3)
  (bind _returnvalue_4 (message `CombatInterface.GetAttackMontages` (`self.GetAvatarActorFromActorInfo`)))
  (bind _output_get (set `self.selectedMontage` (`self.GetRandomTaggedMontageFromArray` _returnvalue_4)))
  (bind (_montage _montagetag) (break `TaggedMontage` _output_get))
  (`AbilityTask_PlayMontageAndWait.CreatePlayMontageAndWaitProxy` "None" _montage 1.0 "None" false
    (:`then`
      (`AbilityTask_WaitGameplayEvent.WaitGameplayEvent` _montagetag null
        (:`EventReceived`
          (bind _returnvalue_5 (message `CombatInterface.GetCombatSocketLocation` (`self.GetAvatarActorFromActorInfo`) _montagetag))
          (`self.SpawnProjectile` _returnvalue_3)
          (`KismetSystemLibrary.DrawDebugSphere` _returnvalue_5 30.0 12 (struct :`G` 1.0 :`B` 0.798421 :`A` 1.0)))))
    (:`OnCompleted`
      (`self.K2_EndAbility` :!label _label))
    (:`OnInterrupted`
      (goto _label))
    (:`OnCancelled`
      (goto _label))))