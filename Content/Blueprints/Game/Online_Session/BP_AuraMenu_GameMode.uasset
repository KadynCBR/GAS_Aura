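; BP_AuraMenu_GameMode is the game mode that manages connected players and their name list in the online session lobby.
; When a new player starts in the lobby level, it stores their BP_AuraMenuController and calls that controller to create the lobby menu and run initial setup.
; UpdateLobby, gated on its PlayerNames input, rebuilds the name list from all stored controllers and pushes it back to each one.
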(event `self.HandleStartingNewPlayer`
  (params (NewPlayer :type "PlayerController Object Reference"))
  ;[1 1 1] Executed if new player enters session
  (bind _returnvalue (`GameplayStatics.GetCurrentLevelName` true))
  (switch `string` _returnvalue
    (:`LobbyLevel`
      (bind _asbp_aura_menu_controller (cast `/Game/Blueprints/Game/Online_Session/BP_AuraMenuController` NewPlayer))
      (`KismetArrayLibrary.Array_Add` (`self.AllConnectedPlayers`) _asbp_aura_menu_controller)
      (`/Game/Blueprints/Game/Online_Session/BP_AuraMenuController.CreateLobbyMenu` _asbp_aura_menu_controller)
      (`/Game/Blueprints/Game/Online_Session/BP_AuraMenuController.InitialSetup` _asbp_aura_menu_controller))))

(event `UpdateLobby`
  (params (PlayerNames :type Boolean))
  (if PlayerNames
    (`KismetArrayLibrary.Array_Clear` (`self.AllPlayerNames`))
    (for _array_element (`self.AllConnectedPlayers`)
      (`KismetArrayLibrary.Array_Add` (`self.AllPlayerNames`) (`/Game/Blueprints/Game/Online_Session/BP_AuraMenuController.PlayerName` _array_element)))
    (for _array_element_2 (`self.AllConnectedPlayers`)
      (if PlayerNames
        (`/Game/Blueprints/Game/Online_Session/BP_AuraMenuController.UpdatePlayerNames` _array_element_2 (`self.AllPlayerNames`))))))

(fn `UserConstructionScript`)