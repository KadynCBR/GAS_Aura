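; Player controller for the multiplayer menu and lobby, handling lobby and character select widgets, player profiles and leaving a session.
; It pulls the profile from the game instance and sends it to the server, where the menu game mode updates player names and character selection.
; Showing either menu blends the camera to the pawn or lobby character view, through a server call on clients.
; Ending the session destroys it and opens the menu level.
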(event `self.ReceiveBeginPlay`
  (if (`self.IsLocalController`)
    (set `self.bShowMouseCursor` true)
    (`WidgetBlueprintLibrary.SetInputMode_UIOnlyEx` self null)))

(event `EndClientSession`
  (`DestroySessionCallbackProxy.DestroySession` self
    (:`then`
      (`GameplayStatics.OpenLevelBySoftObjectPtr` "/Game/Maps/Online_menu/MenuLevel.MenuLevel"))))

(event `CreateLobbyMenu`
  ;[1 1 1] Server tells clients to display lobby menu
  (`self.UI_ShowLobbyMenu`))

(event `InitialSetup`
  (bind _asbp_aura_game_instance (cast `/Game/Blueprints/Game/Online_Session/BP_AuraGameInstance` (`GameplayStatics.GetGameInstance`)))
  (bind _output_get (set `self.PlayerProfile` (`/Game/Blueprints/Game/Online_Session/BP_AuraGameInstance.PlayerProfile` _asbp_aura_game_instance)))
  (`self.Server_UpdateLobby` _output_get))

(event `Server_UpdateLobby`
  (params (PlayerProfile :type "/Game/Blueprints/Online_Menu/S_PlayerProfile Structure"))
  ;[1 1 1] Send our name / player struct to server
  (set `self.PlayerProfile` PlayerProfile)
  (bind _asbp_aura_menu_game_mode (cast `/Game/Blueprints/Game/Online_Session/BP_AuraMenu_GameMode` (`GameplayStatics.GetGameMode`)))
  (`/Game/Blueprints/Game/Online_Session/BP_AuraMenu_GameMode.UpdateLobby` _asbp_aura_menu_game_mode true true))

(event `UpdatePlayerNames`
  (params (PlayerNames :type "Array of String"))
  (bind _widgetlobbymenu (`self.WidgetLobbyMenu`)
    (:`then`
      (`/Game/Blueprints/Online_Menu/WBP_LobbyMenu.ClearPlayerNames` _widgetlobbymenu)
      (`/Game/Blueprints/Online_Menu/WBP_LobbyMenu.UpdatePlayerNames` _widgetlobbymenu PlayerNames))
    (:`else`)))

(event `Server_SetViewTarget_Normal`
  (`self.SetViewTargetWithBlend` (`self.K2_GetPawn`) 0.5))

(event `Server_UpdateSelectedCharacter`
  (params (PlayerProfile :type "/Game/Blueprints/Online_Menu/S_PlayerProfile Structure"))
  (bind _output_get (set `self.PlayerProfile` PlayerProfile))
  (bind _asbp_aura_menu_game_mode (cast `/Game/Blueprints/Game/Online_Session/BP_AuraMenu_GameMode` (`GameplayStatics.GetGameMode`)))
  (`/Game/Blueprints/Game/Online_Session/BP_AuraMenu_GameMode.UpdateCharacterForController` _asbp_aura_menu_game_mode self _output_get))

(event `Server_SetViewTarget_Character`
  (`self.SetViewTargetWithBlend` (`ChildActorComponent.ChildActor` (`/Game/Blueprints/Online_Menu/Lobby/BP_LobbyCharacter.ViewTarget` (`self.LobbyCharacter_BP`))) 0.5))

(fn `SaveSelectedCharacter`
  (params (CharacterName :type Name) (`Player Profile Player Character Class` :type "EPlayerCharacterClass Enum" :default "Aura"))
  (bind _playerprofile_playername (break `/Game/Blueprints/Online_Menu/S_PlayerProfile` (`self.PlayerProfile`)))
  (bind _output_get (set `self.PlayerProfile` (make `/Game/Blueprints/Online_Menu/S_PlayerProfile` _playerprofile_playername CharacterName `Player Profile Player Character Class`)))
  (`self.Server_UpdateSelectedCharacter` _output_get)
  (return))

(fn `UI_ShowCharacterMenu`
  (`/Engine/EditorBlueprintResources/StandardMacros.IsValid` (`self.WidgetCharacterMenu`)
    (:`Is Valid`
      _)
    (:`Is Not Valid`
      (bind _returnvalue (`|CreateWidget` "/Game/Blueprints/Online_Menu/WBP_CharacterSelect.WBP_CharacterSelect_C" self))
      (set `self.WidgetCharacterMenu` _returnvalue)))
  (`UserWidget.AddToViewport` (`self.WidgetCharacterMenu`) 0)
  (`/Engine/EditorBlueprintResources/ActorMacros.Switch Has Authority`
    (:`Authority`
      (`self.SetViewTargetWithBlend` (`ChildActorComponent.ChildActor` (`/Game/Blueprints/Online_Menu/Lobby/BP_LobbyCharacter.ViewTarget` (`self.LobbyCharacter_BP`))) 0.5))
    (:`Remote`
      (`self.Server_SetViewTarget_Character`)))
  (return))

(fn `UI_ShowLobbyMenu`
  (`/Engine/EditorBlueprintResources/StandardMacros.IsValid` (`self.WidgetLobbyMenu`)
    (:`Is Valid`
      _)
    (:`Is Not Valid`
      (bind _returnvalue (`|CreateWidget` "/Game/Blueprints/Online_Menu/WBP_LobbyMenu.WBP_LobbyMenu_C" self))
      (set `self.WidgetLobbyMenu` _returnvalue)))
  (`UserWidget.AddToViewport` (`self.WidgetLobbyMenu`) 0)
  (`/Engine/EditorBlueprintResources/ActorMacros.Switch Has Authority`
    (:`Authority`
      (`self.SetViewTargetWithBlend` (`self.K2_GetPawn`) 0.5))
    (:`Remote`
      (`self.Server_SetViewTarget_Normal`)))
  (return))

(fn `UserConstructionScript`)