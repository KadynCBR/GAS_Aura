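; Base enemy character Blueprint that supplies spawn, dissolve and attack-facing hooks for enemies.
; On BeginPlay a timeline drives the mesh's uniform scale as an intro effect.
; Separate body and weapon dissolve events take a dynamic material instance and animate its Dissolve parameter through their own timelines.
; UpdateFacingTarget sets the Motion Warping "FacingTarget" location once per call, with no continuous tracking.
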(event `self.ReceiveBeginPlay`
  (bind (_direction _newtrack_0) (`Timeline|IntroTimeline`)
    (:`Update`
      (`SceneComponent.SetRelativeScale3D` (`self.Mesh`) (`KismetMathLibrary.MakeVector` _newtrack_0 _newtrack_0 _newtrack_0)))))

(event `self.StartDissolveTimeline`
  (params (DynamicMaterialIsntance :type "MaterialInstanceDynamic Object Reference"))
  (bind (_direction _dissolvetrack) (`Timeline|DissolveTimeline`)
    (:`Update`
      (`MaterialInstanceDynamic.SetScalarParameterValue` DynamicMaterialIsntance "Dissolve" _dissolvetrack))))

(event `self.StartWeaponDissolveTimeline`
  (params (DynamicMaterialIsntance :type "MaterialInstanceDynamic Object Reference"))
  (bind (_direction _dissolvetrack) (`Timeline|WeaponDissolveTimeline`)
    (:`Update`
      (`MaterialInstanceDynamic.SetScalarParameterValue` DynamicMaterialIsntance "Dissolve" _dissolvetrack))))

(event `CombatInterface.UpdateFacingTarget`
  (params (Target :type "Vector Structure (by ref)"))
  ;[1 1 1] If wanted, could do a timeline to update this every frame while timeline is running. allows enemy to rotate to player constantly.
  (`MotionWarpingComponent.AddOrUpdateWarpTargetFromLocation` (`self.MotionWarping`) "FacingTarget" Target))

(fn `UserConstructionScript`)