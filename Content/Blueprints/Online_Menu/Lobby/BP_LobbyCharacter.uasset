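; BP_LobbyCharacter is the character display in the online lobby, showing a player's name and skeletal mesh.
; Multicast events replicate changes to the name text, the CharacterMesh asset and a looping animation played directly on that mesh.
; The name event delegates to a SetPlayerName helper, and the actor has no active BeginPlay, overlap, Tick or construction logic.
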(event `MC_SetPlayerName`
  (params (PlayerName :type Text))
  ;[1 1 1] MultiCast Setting name
  (`self.SetPlayerName` PlayerName))

(event `MC_SetCharacterMesh`
  (params (NewMesh :type "SkeletalMesh Object Reference"))
  ;[1 1 1] Multicast Setting SKM
  (`SkeletalMeshComponent.SetSkeletalMeshAsset` (`self.CharacterMesh`) NewMesh))

(event `MC_PlayMeshAnimation`
  (params (NewAnimToPlay :type "AnimationAsset Object Reference"))
  ;[1 1 1] Multicast Play Anim
  (`SkeletalMeshComponent.PlayAnimation` (`self.CharacterMesh`) NewAnimToPlay true))

(fn `SetPlayerName`
  (params (PlayerName :type Text))
  (`TextRenderComponent.K2_SetText` (`self.PlayerName`) PlayerName)
  (return))

(fn `UserConstructionScript`)